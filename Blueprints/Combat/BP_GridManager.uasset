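; BP_GridManager is a combat grid actor that builds a rectangular tile grid in its construction script.
; It clears and refills the ISMTiles instanced mesh and writes a walkable SGridTile entry per cell into a row-major Tiles array.
; Helper functions convert between XY, index and position using GridWidth, TileSize and Origin, and check bounds.
; It has no runtime event logic.
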(fn `IndexFromXY`
  (params (X :type Integer) (Y :type Integer))
  (returns (Index :type Integer))
  (return (+ X (* Y (`self.GridWidth`)))))

(fn `IsInBounds`
  (params (X :type Integer) (Y :type Integer))
  (returns (bInBounds :type Boolean))
  (return (and (and (>= X 0) (< X (`self.GridWidth`))) (and (>= Y 0) (< Y (`self.GridHeight`))))))

(fn `UserConstructionScript`
  (bind _ism_tiles (`self.ISM_Tiles`))
  (`InstancedStaticMeshComponent.ClearInstances` _ism_tiles)
  (for _index (range (`self.GridHeight`))
    (for _index_2 (range (`self.GridWidth`))
      (bind _world (`self.WorldFromXY` _index_2 _index))
      (`InstancedStaticMeshComponent.AddInstance` _ism_tiles (`KismetMathLibrary.MakeTransform` _world) false)
      (bind _index_3 (`self.IndexFromXY` _index_2 _index))
      (`KismetArrayLibrary.Array_Set` (`|MakeArray` (`self.Tiles`)) _index_3 (make `/Game/TopDownHybrid/Blueprints/Combat/S_GridTile` _index_2 _index _index_3 _world 0 true)))))

(fn `WorldFromXY`
  (params (X :type Integer) (Y :type Integer))
  (returns (World :type "Vector Structure"))
  (bind _tilesize (`self.TileSize`))
  (return (`KismetMathLibrary.MakeVector` (+ (* (`KismetMathLibrary.Conv_IntToDouble` X) _tilesize) (.x (`self.Origin`))) (+ (* _tilesize (`KismetMathLibrary.Conv_IntToDouble` Y)) (.y (`self.Origin`))) (.z (`self.Origin`)))))

(fn `XYFromIndex`
  (params (Index :type Integer))
  (returns (X :type Integer) (Y :type Integer))
  (bind _gridwidth (`self.GridWidth`))
  (return (mod Index _gridwidth) (/ Index _gridwidth)))