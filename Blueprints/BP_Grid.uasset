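; BP_Grid is a grid actor that lays out square tiles and converts between positions and cell indices.
; On BeginPlay, nested loops add one TileInstances instance per cell in local space at TileSize spacing, printing each position.
; GetGridFromWorldPosition floors position to a cell and returns a bounds flag as an integer; GetWorldPositionFormGrid returns cell centers.
; Both conversions ignore the actor's transform, so they assume a grid at the world origin.
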(event `self.ReceiveBeginPlay`
  (`self.GenerateGrid`))

(event `GenerateGrid`
  (for _index (range (`self.GridSizeX`))
    (for _index_2 (range (`self.GridSizeY`))
      (bind _returnvalue (`KismetMathLibrary.MakeVector` (* (`self.TileSize`) _index) (* (`self.TileSize`) _index_2)))
      (`InstancedStaticMeshComponent.AddInstance` (`self.TileInstances`) (`KismetMathLibrary.MakeTransform` _returnvalue) false)
      (`KismetSystemLibrary.PrintString` (`KismetStringLibrary.Conv_VectorToString` _returnvalue)))))

(fn `GetGridFromWorldPosition`
  (params (WorldPosition :type "Vector Structure"))
  (returns (NewX :type Integer) (NewY :type Integer) (Valid :type Integer))
  (bind _tilesize (`self.TileSize`))
  (bind _returnvalue (`KismetMathLibrary.FFloor` (/ (.x WorldPosition) _tilesize)))
  (bind _returnvalue_2 (`KismetMathLibrary.FFloor` (/ (.y WorldPosition) _tilesize)))
  (return _returnvalue _returnvalue_2 (`KismetMathLibrary.Conv_BoolToInt` (and (and (>= _returnvalue 0) (< _returnvalue (`self.GridSizeX`))) (and (>= _returnvalue_2 0) (< _returnvalue_2 (`self.GridSizeY`)))))))

(fn `GetWorldPositionFormGrid`
  (params (GridX :type Integer) (GridY :type Integer))
  (returns (WorldPosition :type "Vector Structure"))
  (bind _tilesize (`self.TileSize`))
  (bind _returnvalue (* 0.5 (`self.TileSize`)))
  (return (`KismetMathLibrary.MakeVector` (+ _returnvalue (* GridX _tilesize)) (+ _returnvalue (* GridY _tilesize)))))

(fn `UserConstructionScript`)