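; BP_Unit is a sprite-based combat unit Blueprint with Enhanced Input, apparently meant for grid movement that is still unfinished.
; BeginPlay adds the hybrid and combat mapping contexts, replicates the Sprite component and caches walk speed.
; Confirm and Select inputs only print debug text.
; MoveToGrid is an empty stub, with its Manhattan-distance check and the grid-manager lookup left disconnected.
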(event `self.ReceiveBeginPlay`
  ;[0.05098 0.05098 0.05098] Init Enhanced Input and set Flipbook to replicated for multiplayer
  (bind _outactors (`GameplayStatics.GetAllActorsOfClass` "/Game/TopDownHybrid/Blueprints/BP_Grid.BP_Grid_C"))
  (`|ExecutionSequence`
    (:`then_0`
      (`self.InitInput`)
      (`ActorComponent.SetIsReplicated` (`self.Sprite`) true)
      ;[0.05098 0.05098 0.05098] Save walk speed from Character Movement Comp
      (set `self.WalkSpeed` (`CharacterMovementComponent.MaxWalkSpeed` (`self.CharacterMovement`))))
    (:`then_1`
      (bind _asplayer_controller (cast `PlayerController` (`GameplayStatics.GetPlayerController` 0)))
      (`EnhancedInputSubsystemInterface.AddMappingContext` (pcsubsystem `EnhancedInputLocalPlayerSubsystem` _asplayer_controller) "/Game/TopDownHybrid/Blueprints/CombatUnit/InputAction/IMC_Combat.IMC_Combat" 0 (struct)))))

(event `EnhancedInput|/Game/TopDownHybrid/Blueprints/CombatUnit/InputAction/IA_Combat_Confirm`
  (params (ActionValue :type Boolean) (ElapsedSeconds :type "Float (double-precision)") (TriggeredSeconds :type "Float (double-precision)") (InputAction :type "InputAction Object Reference" :default "/Game/TopDownHybrid/Blueprints/CombatUnit/InputAction/IA_Combat_Confirm.IA_Combat_Confirm"))
  (:`Triggered`
    (`KismetSystemLibrary.PrintString` "Confirm")))

(event `EnhancedInput|/Game/TopDownHybrid/Blueprints/CombatUnit/InputAction/IA_Combat_Select`
  (params (ActionValue :type Boolean) (ElapsedSeconds :type "Float (double-precision)") (TriggeredSeconds :type "Float (double-precision)") (InputAction :type "InputAction Object Reference" :default "/Game/TopDownHybrid/Blueprints/CombatUnit/InputAction/IA_Combat_Select.IA_Combat_Select"))
  (:`Triggered`
    (`KismetSystemLibrary.PrintString` "Select")))

(fn `InitInput`
  (bind _asplayer_controller (cast `PlayerController` (`self.GetController`))
    (:`then`
      (`EnhancedInputSubsystemInterface.AddMappingContext` (pcsubsystem `EnhancedInputLocalPlayerSubsystem` _asplayer_controller) "/Game/TopDownHybrid/Input/IMC_Hybrid.IMC_Hybrid" 0 (struct))
      (return))
    (:`CastFailed`
      (return))))

(fn `MoveToGrid`
  (params (NewX :type Integer) (NewY :type Integer)))

(fn `UserConstructionScript`)